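; Level trigger actor that starts the player's parachute sequence when the player enters its zone.
; Overlap flags the zone and records entrance velocity, letting a right mouse press begin a deployment timer in Tick that writes the remaining time to the character.
; At the target time, unless touchdown has occurred, it launches the character at a fixed vertical velocity, zeroes gravity and marks the parachute deployed.
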(event EventBeginPlay
  (bind _asthird_person_character (Utilities|Casting|CastToThirdPersonCharacter (Game|GetPlayerCharacter 0)))
  (Variables|Default|Setplayer _asthird_person_character)
  (Input|EnableInput (Game|GetPlayerController (Variables|Default|Getplayer))))

(event Collision|EventActorBeginOverlap
  (params (OtherActor :type Actor%20Object%20Reference))
  (if (not (Variables|/Game/ThirdPersonBP/Blueprints/ThirdPersonCharacter.ThirdPersonCharacter_C|GetparachuteButonPressed? (Variables|Default|Getplayer)))
    (Variables|Default|SetentranceVelocity (Transformation|GetVelocity (Variables|Default|Getplayer)))
    (Variables|/Game/ThirdPersonBP/Blueprints/ThirdPersonCharacter.ThirdPersonCharacter_C|SetenteredParachuteZone (Variables|Default|Getplayer) true)))

(event EventTick
  (params (DeltaSeconds :type Float%20%28single-precision%29))
  (if (not (Variables|/Game/ThirdPersonBP/Blueprints/ThirdPersonCharacter.ThirdPersonCharacter_C|GetparachuteDeployed (Variables|Default|Getplayer)))
    (if (Variables|/Game/ThirdPersonBP/Blueprints/ThirdPersonCharacter.ThirdPersonCharacter_C|GetparachuteButonPressed? (Variables|Default|Getplayer))
      (bind _output_get (Variables|Default|SetdeploymentTime (+ (Variables|Default|GetdeploymentTime) (Utilities|Time|GetWorldDeltaSeconds))))
      (Variables|/Game/ThirdPersonBP/Blueprints/ThirdPersonCharacter.ThirdPersonCharacter_C|SetparachuteDeploymentTime (Variables|Default|Getplayer) (- (Variables|Default|GettargetTime) _output_get))
      (Variables|Default|SettimeOfDeployment (Utilities|Time|GetGameTimeinSeconds))
      (if (>= (Variables|Default|GetdeploymentTime) (Variables|Default|GettargetTime))
        (if (not (Variables|/Game/ThirdPersonBP/Blueprints/ThirdPersonCharacter.ThirdPersonCharacter_C|GetparachuteTouchdown (Variables|Default|Getplayer)))
          (Character|LaunchCharacter (Variables|Default|Getplayer) (Math|Vector|MakeVector 0.0 0.0 (Variables|Default|GettargetEndVelocity)) false true)
          (Variables|/Script/Engine.CharacterMovementComponent|SetGravityScale (Variables|/Script/Engine.Character|GetCharacterMovement (Variables|Default|Getplayer)) 0.0)
          (Variables|/Game/ThirdPersonBP/Blueprints/ThirdPersonCharacter.ThirdPersonCharacter_C|SetparachuteDeployed (Variables|Default|Getplayer) true)
          (Variables|Default|SetdeploymentTime 0.0))))))

(event Input|MouseEvents|RightMouseButton
  (params (Key :type Key%20Structure))
  (:Pressed
    (if (Variables|/Game/ThirdPersonBP/Blueprints/ThirdPersonCharacter.ThirdPersonCharacter_C|GetenteredParachuteZone (Variables|Default|Getplayer))
      (Variables|/Game/ThirdPersonBP/Blueprints/ThirdPersonCharacter.ThirdPersonCharacter_C|SetparachuteButonPressed? (Variables|Default|Getplayer) true))))

(fn ConstructionScript)