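; Trigger box Blueprint that turns a cube a fixed pink while the player character is inside it.
; The construction script creates a dynamic material instance and assigns it to the first Cube_Blueprint found in the level.
; Overlap events set a flag that makes Tick set the color and print a normalized horizontal distance from the attach parent to the player.
; A distance-driven color lerp is left unconnected.
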(event EventBeginPlay)

(event Collision|EventActorBeginOverlap
  (params (OtherActor :type Actor%20Object%20Reference))
  (if (== OtherActor (Game|GetPlayerCharacter 0))
    (Variables|Default|SetisInCollider true)))

(event Collision|EventActorEndOverlap
  (params (OtherActor :type Actor%20Object%20Reference))
  (if (== OtherActor (Game|GetPlayerCharacter 0))
    (Variables|Default|SetisInCollider false)))

(event EventTick
  (params (DeltaSeconds :type Float%20%28single-precision%29))
  (if (Variables|Default|GetisInCollider)
    (Development|PrintString (Utilities|String|ToString(Float) (|((X-Y)/Z) (Transformation|GetHorizontalDistanceTo (Actor|GetAttachParentActor) (Game|GetPlayerCharacter 0)) 3e+02 3e+02)))
    (Rendering|Material|SetVectorParameterValue (Variables|Default|GetcubeMat) "Color" "(R=1.000000,G=0.417225,B=0.653000,A=1.000000)" :!class /Script/Engine.MaterialInstanceDynamic)))

(fn ConstructionScript
  (bind _returnvalue (Rendering|Material|CreateDynamicMaterialInstance "/Game/materials/cubeMat.cubeMat" :!class /Script/Engine.KismetMaterialLibrary))
  (Variables|Default|SetcubeMat _returnvalue)
  (bind _outactors (Actor|GetAllActorsOfClass "/Game/levelPieceBP/Cube_Blueprint.Cube_Blueprint_C"))
  (Rendering|Material|SetMaterial (Variables|/Script/Engine.StaticMeshActor|GetStaticMeshComponent (Utilities|Array|Get(acopy) _outactors)) 0 (Variables|Default|GetcubeMat)))

(fn NewFunction0
  (Development|PrintString "Hello"))