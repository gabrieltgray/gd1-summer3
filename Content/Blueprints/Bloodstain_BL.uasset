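; Bloodstain interactable that removes floor meshes when the player presses E nearby.
; A box overlap with ThirdPersonCharacter shows a text prompt and enables input, and leaving reverses both.
; E sets each static mesh component on the Floors actor to simulated, physics-only collision, then destroys it immediately.
; After a one-second delay, a second pass toggles activation and visibility on any remaining meshes.
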(event OnComponentBeginOverlap(Box)
  (params (OverlappedComponent :type Primitive%20Component%20Object%20Reference) (OtherActor :type Actor%20Object%20Reference) (OtherComp :type Primitive%20Component%20Object%20Reference) (OtherBodyIndex :type Integer) (bFromSweep :type Boolean) (SweepResult :type Hit%20Result%20Structure%20%28by%20ref%29))
  (Utilities|Casting|CastToThirdPersonCharacter OtherActor)
  (Rendering|SetVisibility (Variables|Default|GetTextRender) true false)
  (Input|EnableInput (Game|GetPlayerController 0)))

(event OnComponentEndOverlap(Box)
  (params (OverlappedComponent :type Primitive%20Component%20Object%20Reference) (OtherActor :type Actor%20Object%20Reference) (OtherComp :type Primitive%20Component%20Object%20Reference) (OtherBodyIndex :type Integer))
  (Utilities|Casting|CastToThirdPersonCharacter OtherActor)
  (Rendering|SetVisibility (Variables|Default|GetTextRender) false false)
  (Input|DisableInput (Game|GetPlayerController 0)))

(event EventBeginPlay)

(event EventTick
  (params (DeltaSeconds :type Float%20%28single-precision%29)))

(event Input|KeyboardEvents|E
  (params (Key :type Key%20Structure))
  (bind _floors (Variables|Default|GetFloors))
  (bind _returnvalue (Actor|GetComponentsByClass _floors "/Script/Engine.StaticMeshComponent"))
  (:Pressed
    (for _array_element _returnvalue
      (Physics|SetSimulatePhysics _array_element true)
      (Collision|SetCollisionEnabled _array_element "PhysicsOnly")
      (Components|DestroyComponent _array_element))
    (Utilities|FlowControl|Delay 1.0)
    (for _array_element_2 _returnvalue
      (Components|Activation|ToggleActive _array_element_2)
      (Rendering|ToggleVisibility _array_element_2 false))))

(fn ConstructionScript)